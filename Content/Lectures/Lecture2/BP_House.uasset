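; BP_House is a house actor that switches a referenced light on or off when the first-person player character overlaps it.
; On BeginPlay it caches the player as BP_FirstPersonCharacter.
; Each begin-overlap from that character flips an Inside flag and sets the PointLight intensity on LightRef to lit or zero accordingly.
; No end-overlap is handled, so the light alternates on successive entries rather than tracking actual presence.
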(event EventBeginPlay
  (bind _asbp_first_person_character (Utilities|Casting|CastToBP_FirstPersonCharacter (Game|GetPlayerCharacter 0)))
  (Variables|Default|SetAs%20BP%20First%20Person%20Character _asbp_first_person_character))

(event Collision|EventActorBeginOverlap
  (params (OtherActor :type Actor%20Object%20Reference))
  (if (== OtherActor (Variables|Default|GetAs%20BP%20First%20Person%20Character))
    (bind _output_get (Variables|Default|SetInside (not (Variables|Default|GetInside))))
    (if _output_get
      (Rendering|Components|Light|SetIntensity (Variables|/Game/Lectures/Lecture2/BP_Light.BP_Light_C|GetPointLight (Variables|Default|GetLightRef)) 1e+03)
      (else
        (Rendering|Components|Light|SetIntensity (Variables|/Game/Lectures/Lecture2/BP_Light.BP_Light_C|GetPointLight (Variables|Default|GetLightRef)) 0.0)))))

(event EventTick
  (params (DeltaSeconds :type Float%20%28single-precision%29)))

(fn ConstructionScript)