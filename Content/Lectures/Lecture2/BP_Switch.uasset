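; BP_Switch is a switch actor that recolors a referenced light when the first-person player touches it while holding a key.
; On BeginPlay it caches the player character as BP_FirstPersonCharacter.
; On overlap it checks that the actor is that player and that HasKey is set, then gives the point light of LİghtRef a random color.
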(event EventBeginPlay
  (bind _asbp_first_person_character (Utilities|Casting|CastToBP_FirstPersonCharacter (Game|GetPlayerCharacter 0)))
  (Variables|Default|SetAs%20BP%20First%20Person%20Character _asbp_first_person_character))

(event Collision|EventActorBeginOverlap
  (params (OtherActor :type Actor%20Object%20Reference))
  (if (== (Variables|Default|GetAs%20BP%20First%20Person%20Character) OtherActor)
    (if (Variables|/Game/FirstPerson/Blueprints/BP_FirstPersonCharacter.BP_FirstPersonCharacter_C|GetHasKey? (Variables|Default|GetAs%20BP%20First%20Person%20Character))
      (Rendering|Components|Light|SetLightColor (Variables|/Game/Lectures/Lecture2/BP_Light.BP_Light_C|GetPointLight (Variables|Default|GetLİghtRef)) (Utilities|Struct|MakeLinearColor (Math|Random|RandomFloat) (Math|Random|RandomFloat) (Math|Random|RandomFloat) 1.0) true))))

(event EventTick
  (params (DeltaSeconds :type Float%20%28single-precision%29)))

(fn ConstructionScript)